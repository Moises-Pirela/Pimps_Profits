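; BP_Pimp is an interactable character Blueprint that shows an on-screen interaction prompt when focused.
; On BeginPlay it creates a UI_InteractionPrompt widget for player 0, adds it to the viewport and hides it.
; PnPInteraction focus events show the prompt with hardcoded placeholder-looking text, then hide it when focus ends.
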(event OnBeginFocus(PnPInteraction)
  (params (Interactable :type Actor%20Object%20Reference))
  (bind _interactionprompt (Variables|Default|GetInteractionPrompt))
  (Utilities|IsValid _interactionprompt
    (:Is%20Valid
      (Widget|SetVisibility _interactionprompt "Visible")
      (Default|SetDisplayText _interactionprompt "ghello"))))

(event OnEndFocus(PnPInteraction)
  (params (Interactable :type Actor%20Object%20Reference))
  (bind _interactionprompt (Variables|Default|GetInteractionPrompt))
  (Utilities|IsValid _interactionprompt
    (:Is%20Valid
      (Widget|SetVisibility _interactionprompt "Hidden"))))

(event EventBeginPlay
  (bind _returnvalue (UserInterface|CreateWidget "/Game/_PNP/UI/Blueprints/UI_InteractionPrompt.UI_InteractionPrompt_C" (Class|GameplayStatics|GetPlayerControllerfromID)))
  (bind _output_get (Variables|Default|SetInteractionPrompt _returnvalue))
  (Utilities|IsValid _output_get
    (:Is%20Valid
      (UserInterface|Viewport|AddtoViewport _output_get 0)
      (Widget|SetVisibility (Variables|Default|GetInteractionPrompt) "Hidden"))))

(fn ConstructionScript)